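; Base physics pickup actor that lets the player grab, carry, drop and inspect an object.
; Pickup constrains MainMash to a camera-attached Root, either at the clicked point (Accurate) or an offset pivot, and impacts briefly free the linear limits.
; An optional swept duplicate mesh replaces the visible one when it would pass through walls.
; Inspection locks player movement, enables post-process and rotates the object by input, with empty hooks for children like BP_PickUp_Hard.
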(event `HitCustom`
  (params (HitComponent :type "PrimitiveComponent Object Reference") (OtherActor :type "Actor Object Reference") (OtherComp :type "PrimitiveComponent Object Reference") (NormalImpulse :type "Vector Structure") (Hit :type "HitResult Structure (by ref)"))
  (bind _physicsconstraint (`self.PhysicsConstraint`))
  ;[1 1 1] Hit
  (if (`self.IgnoreHit?`)
    _
    (elif (`self.Attach`)
      (set `self.HitActive` true)
      (`PhysicsConstraintComponent.SetLinearXLimit` _physicsconstraint "LCM_Free" 0.0)
      (`PhysicsConstraintComponent.SetLinearYLimit` _physicsconstraint "LCM_Free" 0.0)
      (`PhysicsConstraintComponent.SetLinearZLimit` _physicsconstraint "LCM_Free" 0.0)
      (`self.Free`)
      (`KismetSystemLibrary.RetriggerableDelay` (`self.RecoveryFromHit`))
      (`|ExecutionSequence`
        (:`then_0`
          (`PhysicsConstraintComponent.SetLinearXLimit` _physicsconstraint "LCM_Locked" 0.0)
          (`PhysicsConstraintComponent.SetLinearYLimit` _physicsconstraint "LCM_Locked" 0.0)
          (`PhysicsConstraintComponent.SetLinearZLimit` _physicsconstraint "LCM_Locked" 0.0)
          (`self.Lock`)
          (set `self.HitActive` false))))))

(event `Lock`
  ;[1 1 1] Hit
  ;;[1 1 1] Used in child classes. BP_PickUp_Hard
)

(event `Free`
  ;[1 1 1] Hit
  ;;[1 1 1] Used in child classes. BP_PickUp_Hard
)

(event `self.ReceiveBeginPlay`
  (bind _root (`self.Root`))
  ;[1 1 1] BeginPlay
  (`/Engine/EditorBlueprintResources/StandardMacros.IsValid` (`self.PhysicsConstraint`)
    (:`Is Valid`
      (`|ExecutionSequence`
        (:`then_0`
          (add `PrimitiveComponent.OnComponentHit` (`self.MainMash`) (`|CreateDelegate` :!event `HitCustom`))
          (if (`|EnumEquality` (`PrimitiveComponent.GetCollisionEnabled` (`self.MainMash`)) "QueryAndPhysics")
            (`PrimitiveComponent.SetSimulatePhysics` (`self.MainMash`) (`self.StartPhysics`)))
          (`SceneComponent.SetAbsolute` _root false true false)
          (`SceneComponent.K2_SetWorldRotation` :`self` _root))
        (:`then_1`
          (if (`self.FixWallPassThrough`)
            (add `PrimitiveComponent.OnComponentHit` (`self.SweepMesh`) (`|CreateDelegate` :!event `SweepMeshHit`))))))))

(event `SweepMeshHit`
  (params (HitComponent :type "PrimitiveComponent Object Reference") (OtherActor :type "Actor Object Reference") (OtherComp :type "PrimitiveComponent Object Reference") (NormalImpulse :type "Vector Structure") (Hit :type "HitResult Structure (by ref)"))
  (bind _mainmash (`self.MainMash`))
  (bind _returnvalue (`SceneComponent.K2_GetComponentLocation` (`self.MainMash`)))
  (bind (_bblockinghit _binitialoverlap _time _distance _location _impactpoint _normal _impactnormal) (`GameplayStatics.BreakHitResult` (`self.Hit`)))
  (bind _returnvalue_2 (`KismetMathLibrary.Vector_Distance` _returnvalue _impactpoint))
  ;[1 1 1] Hit
  ;;[0 0 0] FixWallPassThrough
  (if (`self.Attach`)
    (`KismetSystemLibrary.Delay` 0.0)
    (if (> (`KismetMathLibrary.Vector_Distance` (`SceneComponent.K2_GetComponentLocation` (`self.MainMash`)) (`SceneComponent.K2_GetComponentLocation` (`self.SweepMesh`))) 20.0)
      (`/Engine/EditorBlueprintResources/StandardMacros.DoOnce` false :!label _label
        (:`Completed`
          (set `self.Hit` Hit)
          (`|ExecutionSequence`
            (:`then_0`
              (set `self.FixWallPassActive` true)
              (`SceneComponent.SetVisibility` (`self.SweepMesh`) true false)
              (`SceneComponent.SetVisibility` _mainmash false false)
              (`PrimitiveComponent.SetCollisionResponseToAllChannels` _mainmash "ECR_Ignore")
              (set `self.TickForSweep` false)
              (`self.SweepMeshOn`))
            (:`then_1`
              (goto _label_2 :!via `Open`))
            (:`then_2`
              (`/Engine/EditorBlueprintResources/StandardMacros.Gate` true :!label _label_2
                (:`Exit`
                  (`|ExecutionSequence`
                    (:`then_0`
                      (if (and (< (`KismetMathLibrary.Vector_Distance` _returnvalue (+ _impactpoint (* _impactnormal 5.0))) _returnvalue_2) (> _returnvalue_2 25.0))
                        (`|ExecutionSequence` :!label _label_3
                          (:`then_0`
                            (`|ExecutionSequence`
                              (:`then_0`
                                (goto _label_2 :!via `Close`))
                              (:`then_1`
                                (set `self.FixWallPassActive` false))
                              (:`then_2`
                                (goto _label :!via `Reset`))))
                          (:`then_1`
                            (`SceneComponent.SetVisibility` (`self.SweepMesh`) false false)
                            (`SceneComponent.SetVisibility` (`self.MainMash`) true false)
                            (`self.SweepMeshOff`)
                            (if (`self.Attach`)
                              (`self.DefaultCollision`)
                              (`PrimitiveComponent.SetCollisionResponseToChannel` (`self.MainMash`) "ECC_Pawn" "ECR_Ignore")
                              (set `self.TickForSweep` true))))))
                    (:`then_1`
                      (`KismetSystemLibrary.Delay` 0.0)
                      (goto _label_2))))))))))))

(event `SweepMeshOn`
  ;[1 1 1] Hit
  ;;[0 0 0] FixWallPassThrough
  ;;;[1 1 1] Used in child classes. (BP_PickUp_Hard)
)

(event `SweepMeshOff`
  ;[1 1 1] Hit
  ;;[0 0 0] FixWallPassThrough
  ;;;[1 1 1] Used in child classes. (BP_PickUp_Hard)
)

(event `StopSweep`
  ;[1 1 1] Hit
  ;;[0 0 0] FixWallPassThrough
  (`SceneComponent.K2_SetWorldTransform` (`self.MainMash`) (`SceneComponent.K2_GetComponentToWorld` (`self.SweepMesh`)) false true)
  (goto _label_3))

(event `self.ReceiveTick`
  (params (DeltaSeconds :type "Float (single-precision)"))
  ;[1 1 1] EventTick
  (if (and (`self.TickForSweep`) (`self.FixWallPassThrough`))
    (`SceneComponent.K2_SetWorldTransform` (`self.SweepMesh`) (`SceneComponent.K2_GetComponentToWorld` (`self.MainMash`)) true false)))

(event `CustomAttach`
  (bind _mainmash (`self.MainMash`))
  (bind _mainmash_2 (`self.MainMash`))
  (bind (_last_location _last_rotation) (`KismetMathLibrary.BreakTransform` (`self.Last`)))
  (bind (_inttransform_location _inttransform_rotation) (`KismetMathLibrary.BreakTransform` (`self.IntTransform`)))
  (bind _beforeaction_location (`KismetMathLibrary.BreakTransform` (`self.BeforeAction`)))
  (bind (_beforeaction_location_2 _beforeaction_rotation) (`KismetMathLibrary.BreakTransform` (`self.BeforeAction`)))
  (bind _physicsconstraint (`self.PhysicsConstraint`))
  (bind _mainmash_3 (`self.MainMash`))
  (bind (_beforeaction_location_3 _beforeaction_rotation_2) (`KismetMathLibrary.BreakTransform` (`self.BeforeAction`)))
  (bind _mainmash_4 (`self.MainMash`))
  (bind _transformcomponent (`PlayerCameraManager.TransformComponent` (`GameplayStatics.GetPlayerCameraManager` 0)))
  (bind _transformcomponent_2 (`PlayerCameraManager.TransformComponent` (`GameplayStatics.GetPlayerCameraManager` 0)))
  (bind _transformcomponent_3 (`PlayerCameraManager.TransformComponent` (`GameplayStatics.GetPlayerCameraManager` 0)))
  (bind _returnvalue (`SceneComponent.K2_GetComponentLocation` _transformcomponent_2))
  ;[1 1 1] Pickup
  (set `self.Attach` true :!label _label_4)
  (`self.EnableInput` (`GameplayStatics.GetPlayerController` 0))
  (`/Engine/EditorBlueprintResources/StandardMacros.IsValid` (`self.PhysicsConstraint`)
    (:`Is Valid`
      ;;[1 1 1] For stability.
      (if (not (or (`SceneComponent.IsSimulatingPhysics` _mainmash "None") (`self.Rotate`)))
        (`KismetSystemLibrary.Delay` 0.0)
        (`PrimitiveComponent.SetSimulatePhysics` _mainmash true))
      (`|ExecutionSequence`
        (:`then_0`
          (`PhysicsConstraintComponent.BreakConstraint` (`self.PhysicsConstraint`))
          ;;[1 1 1] Memorise the default collision
          (`KismetArrayLibrary.Array_Clear` (`self.IntCollision`))
          (bind _enumvalue (foreach `ECollisionChannel` false)
            (:`LoopBody`
              (`KismetArrayLibrary.Array_Add` (`self.IntCollision`) (`PrimitiveComponent.GetCollisionResponseToChannel` (`self.MainMash`) _enumvalue)))
            (:`then`
              (`PrimitiveComponent.SetCollisionResponseToChannel` (`self.MainMash`) "ECC_Pawn" "ECR_Ignore")
              (set `self.BeforeAction` (`SceneComponent.K2_GetComponentToWorld` (`self.MainMash`)))
              (set `SceneComponent.bAbsoluteLocation` true (`self.MainMash`))
              (set `SceneComponent.bAbsoluteLocation` true (`self.PhysicsConstraint`))
              (if (`self.FixWallPassThrough`)
                (set `self.TickForSweep` true)
                (`SceneComponent.SetVisibility` (`self.SweepMesh`) false false))
              (if (`self.Accurate`)
                ;;[0 0 0] Accurate
                (if (`self.Rotate`)
                  (`SceneComponent.K2_SetWorldLocationAndRotation` _mainmash_3 _last_location _last_rotation false true)
                  (`PrimitiveComponent.SetCollisionResponseToAllChannels` _mainmash_3 "ECR_Overlap") ; To prevent nearby meshes from flying off
                )
                (`SceneComponent.K2_SetWorldLocation` _physicsconstraint (`.ImpactPoint` (`GameplayStatics.BreakHitResult` (`self.HitClick`))) false true)
                (`SceneComponent.K2_SetWorldLocation` (`self.Root`) (`.ImpactPoint` (`GameplayStatics.BreakHitResult` (`self.HitClick`))) false true)
                (`PrimitiveComponent.SetSimulatePhysics` _mainmash_2 true)
                (`PhysicsConstraintComponent.SetConstrainedComponents` (`self.PhysicsConstraint`) (`self.Root`) "None" _mainmash_2 "None")
                (if (`self.Rotate`)
                  ;;;[1 1 1] Solves a lot of problems when returning from inspection
                  (`SceneComponent.K2_SetWorldLocation` (`self.PhysicsConstraint`) (+ _returnvalue (* (`SceneComponent.GetForwardVector` _transformcomponent_2) (`KismetMathLibrary.Vector_Distance` _returnvalue _beforeaction_location))) false true)
                  (`SceneComponent.K2_SetWorldLocation` (`self.Root`) (+ _returnvalue (* (`SceneComponent.GetForwardVector` _transformcomponent_2) (`KismetMathLibrary.Vector_Distance` _returnvalue _beforeaction_location))) false true)
                  (else
                    (`SceneComponent.K2_AttachToComponent` (`self.Root`) _transformcomponent "None" "KeepWorld" "KeepWorld" "KeepWorld" true)
                    (`SceneComponent.K2_AttachToComponent` _physicsconstraint _transformcomponent "None" "KeepWorld" "KeepWorld" "KeepWorld" true)))
                (`|ExecutionSequence`
                  (:`then_0`
                    (if (`self.Rotate`)
                      ;;;[1 1 1] Returning from where you got it
                      (`KismetSystemLibrary.Delay` 0.0)
                      (`SceneComponent.K2_SetWorldLocationAndRotation` (`self.MainMash`) _beforeaction_location_2 _beforeaction_rotation false true)
                      (`self.DefaultCollision`)
                      (`PrimitiveComponent.SetCollisionResponseToChannel` (`self.MainMash`) "ECC_Pawn" "ECR_Ignore")
                      (else
                        (set `self.Last` (`SceneComponent.K2_GetComponentToWorld` (`self.MainMash`)))))))
                (else
                  ;;[1 1 1] Ignore other physical subjects.
                  (if (not (`self.IgnoreCamera?`))
                    (`PrimitiveComponent.SetCollisionResponseToChannel` (`self.MainMash`) "ECC_PhysicsBody" "ECR_Ignore"))
                  (`SceneComponent.K2_SetWorldLocation` (`self.Root`) (`self.AttachLocation`) false true)
                  (`SceneComponent.K2_SetWorldLocation` (`self.PhysicsConstraint`) (`self.AttachLocation`) false true)
                  (`SceneComponent.K2_AttachToComponent` (`self.Root`) _transformcomponent_3 "None" "KeepWorld" "KeepRelative" "KeepWorld" true)
                  (`SceneComponent.K2_AttachToComponent` (`self.PhysicsConstraint`) _transformcomponent_3 "None" "KeepWorld" "KeepRelative" "KeepWorld" true)
                  (`SceneComponent.K2_AttachToComponent` (`self.MainMash`) (`self.Root`) "None" "KeepWorld" "KeepWorld" "KeepWorld" true)
                  (set `SceneComponent.bAbsoluteLocation` false (`self.MainMash`))
                  (`SceneComponent.K2_SetRelativeLocationAndRotation` _mainmash_4 _inttransform_location _inttransform_rotation false true) ; Creating a new pivot
                  (`PrimitiveComponent.SetSimulatePhysics` _mainmash_4 true)
                  (`PhysicsConstraintComponent.SetConstrainedComponents` (`self.PhysicsConstraint`) (`self.Root`) "None" _mainmash_4 "None")
                  ;;[1 1 1] Returning from where you got it
                  (`KismetSystemLibrary.Delay` 0.0)
                  (`SceneComponent.K2_SetWorldLocationAndRotation` _mainmash_4 _beforeaction_location_3 _beforeaction_rotation_2 false true)
                  (`self.HitCustom` null null null (0.0 0.0 0.0) (`GameplayStatics.MakeHitResult` false))
                  ;;[1 1 1] Returning collisions
                  (`KismetSystemLibrary.RetriggerableDelay` 0.1)
                  (if (`self.Attach`)
                    (`self.DefaultCollision`)
                    (`PrimitiveComponent.SetCollisionResponseToChannel` (`self.MainMash`) "ECC_Pawn" "ECR_Ignore")))))))
        (:`then_1`
          (`KismetSystemLibrary.Delay` 0.0)
          (`PrimitiveComponent.WakeAllRigidBodies` (`self.MainMash`)))))))

(event `/Game/PhysicalS/Misk/i_Pickup.Pickup`
  (params (Accurate :type Boolean) (Hit :type "HitResult Structure") (HideHandIco :type Boolean))
  (bind _returnvalue (not Accurate))
  (bind _physicsconstraint (`self.PhysicsConstraint`))
  ;[1 1 1] Pickup
  (`|ExecutionSequence`
    (:`then_0`
      (set `self.Accurate` Accurate)
      (set `self.HitClick` Hit)
      ;;[1 1 1] Adding stability to items
      (if (<= (`self.SuppressionInertia`) 1.0)
        (goto _label_4)
        (else
          (`PhysicsConstraintComponent.SetAngularDriveMode` _physicsconstraint (select `bool` Accurate :`false` "TwistAndSwing" :`true` "SLERP" :!type "EAngularDriveMode Enum"))
          (`PhysicsConstraintComponent.SetAngularVelocityDriveTwistAndSwing` _physicsconstraint _returnvalue _returnvalue)
          (`PhysicsConstraintComponent.SetOrientationDriveTwistAndSwing` _physicsconstraint _returnvalue _returnvalue)
          (`PhysicsConstraintComponent.SetAngularDriveParams` _physicsconstraint 50.0 (`KismetMathLibrary.SelectFloat` 1.0 (`self.SuppressionInertia`) Accurate) 0.0)
          (goto _label_4))))
    (:`then_1`
      (`self.ED_Pickup`))))

(event `/Game/PhysicalS/Misk/i_Pickup.Drop`
  (bind _returnvalue (`GameplayStatics.GetPlayerController` 0))
  (bind _mainmash (`self.MainMash`))
  ;[1 1 1] Drop
  (`|ExecutionSequence`
    (:`then_0`
      (if (`self.FixWallPassThrough`)
        (`self.StopSweep`))
      (if (or (`self.Rotate`) (`TimelineComponent.IsPlaying` (`self.Timeline_In`)))
        (set `self.Rotate` false)
        (`TimelineComponent.Stop` (`self.Timeline_In`))
        (`TimelineComponent.Stop` (`self.Timeline_Out`))
        (`Controller.SetIgnoreMoveInput` _returnvalue false)
        (`Controller.SetIgnoreLookInput` _returnvalue false)
        (`PrimitiveComponent.SetSimulatePhysics` _mainmash true)
        (`PrimitiveComponent.SetRenderCustomDepth` _mainmash false)
        (set `PostProcessVolume.bEnabled` false (`/Game/PhysicalS/BP/Character/PC_PIS.PP_Playroom` (cast `/Game/PhysicalS/BP/Character/PC_PIS` (`GameplayStatics.GetPlayerController` 0) :!pure true))))
      (set `self.Attach` false)
      (`PhysicsConstraintComponent.BreakConstraint` (`self.PhysicsConstraint`))
      (`|ExecutionSequence`
        (:`then_0`
          (`self.DefaultCollision`)
          (`KismetArrayLibrary.Array_Clear` (`self.IntCollision`))
          (`self.DisableInput` (`GameplayStatics.GetPlayerController` 0))
          (`Widget.SetVisibility` (`/Game/PhysicalS/Widgets/w_Hud.Center` (`/Game/PhysicalS/BP/Character/PC_PIS.Hud` (cast `/Game/PhysicalS/BP/Character/PC_PIS` (`GameplayStatics.GetPlayerController` 0) :!pure true))) "SelfHitTestInvisible"))
        (:`then_1`
          (`KismetSystemLibrary.Delay` 0.0)
          (`PrimitiveComponent.WakeAllRigidBodies` (`self.MainMash`)))
        (:`then_2`
          (`KismetSystemLibrary.RetriggerableDelay` 1.0)
          (if (not (`self.Attach`))
            (set `self.TickForSweep` false)
            (`SceneComponent.K2_DetachFromComponent` (`self.Root`) "KeepWorld" "KeepRelative" "KeepWorld" true)))))
    (:`then_1`
      (`self.ED_Drop`))))

(event `Inspection`
  (bind _hud (`/Game/PhysicalS/BP/Character/PC_PIS.Hud` (cast `/Game/PhysicalS/BP/Character/PC_PIS` (`GameplayStatics.GetPlayerController` 0) :!pure true)))
  ;[1 1 1] Rotate/Inspection
  ;;[0 0 0] Click
  (if (`self.DenyInspection`) :!label _label_5
    _
    (elif (`self.Rotate`)
      (`self.RotateOff`)
      (`Widget.SetVisibility` (`/Game/PhysicalS/Widgets/w_Hud.Center` _hud) "SelfHitTestInvisible")
      (else
        ;;;[1 1 1] IN
        (if false
          (`/Game/PhysicalS/Widgets/w_Hud.Hint` _hud "You are already holding the object gently. Inspecting and turning the object may have unexpected consequences.")
          (elif (or (`TimelineComponent.IsPlaying` (`self.Timeline_In`)) (`self.Rotate`))
            _
            (elif (or (and (`self.CheckHitBeforeRot?`) (`self.HitActive`)) (and (not (`self.TickForSweep`)) (`self.FixWallPassThrough`)))
              (`/Game/PhysicalS/Widgets/w_Hud.Hint` _hud "The object concerns something. You will not be able to freely rotate the object in this state.")
              (else
                (`self.RotateOn`)
                (`Widget.SetVisibility` (`/Game/PhysicalS/Widgets/w_Hud.Center` _hud) "Collapsed")))))))))

(event `InputAction|Inspection`
  (params (Key :type "Key Structure"))
  ;[1 1 1] Rotate/Inspection
  ;;[0 0 0] Click
  (:`Pressed`
    (goto _label_5)))

(event `RotateOff`
  (bind (_returnvalue_location _returnvalue_rotation) (`KismetMathLibrary.BreakTransform` (`self.GetTransform`)))
  (bind _returnvalue (`GameplayStatics.GetPlayerController` 0))
  (bind (_beforeaction_location _beforeaction_rotation) (`KismetMathLibrary.BreakTransform` (`self.BeforeAction`)))
  ;[1 1 1] Rotate/Inspection
  ;;[0 0 0] Out
  (if (`self.Accurate`)
    (bind (_direction _newtrack_0) (`Timeline|Timeline_Out` :!via `PlayFromStart` :!label _label_6)
      (:`Update`
        (`SceneComponent.K2_SetWorldLocationAndRotation` (`self.MainMash`) (`KismetMathLibrary.VLerp` _returnvalue_location _beforeaction_location _newtrack_0) (`KismetMathLibrary.RLerp` _returnvalue_rotation _beforeaction_rotation _newtrack_0 true) true false))
      (:`Finished`
        (`self.CustomAttach` :!label _label_7)
        (set `self.Rotate` false)
        ;;;[1 1 1] PP Effect Off
        (`PrimitiveComponent.SetRenderCustomDepth` (`self.MainMash`) false)
        (set `PostProcessVolume.bEnabled` false (`/Game/PhysicalS/BP/Character/PC_PIS.PP_Playroom` (cast `/Game/PhysicalS/BP/Character/PC_PIS` (`GameplayStatics.GetPlayerController` 0) :!pure true)))
        (`Controller.SetIgnoreMoveInput` _returnvalue false)
        (`Controller.SetIgnoreLookInput` _returnvalue false)))
    (else
      (cast `/Game/PhysicalS/BP/BP_PickUp_Hard` self
        (:`then`
          (goto _label_7))
        (:`CastFailed`
          (goto _label_6 :!via `PlayFromStart`))))))

(event `LookUp`
  (params (DeltaY :type "Float (double-precision)"))
  ;[1 1 1] Rotate/Inspection
  ;;[1 1 1] InputMouse
  (if (`self.Rotate`)
    (`SceneComponent.K2_AddLocalRotation` (`self.DefaultSceneRoot`) (`KismetMathLibrary.MakeRotator` 0.0 DeltaY) false false)))

(event `InputAxis|LookUp` :consume false
  (params (AxisValue :type "Float (single-precision)"))
  ;[1 1 1] Rotate/Inspection
  ;;[1 1 1] InputMouse
  (`self.LookUp` AxisValue))

(event `RotateOn`
  (bind _returnvalue (`GameplayStatics.GetPlayerController` 0))
  (bind _mainmash (`self.MainMash`))
  (bind _mainmash_2 (`self.MainMash`))
  (bind (_beforeaction_location _beforeaction_rotation) (`KismetMathLibrary.BreakTransform` (`self.BeforeAction`)))
  ;[1 1 1] Rotate/Inspection
  ;;[0 0 0] In
  (`Controller.SetIgnoreMoveInput` _returnvalue true)
  (`Controller.SetIgnoreLookInput` _returnvalue true)
  ;;;[1 1 1] Disabling physics
  (`PhysicsConstraintComponent.BreakConstraint` (`self.PhysicsConstraint`))
  (`PrimitiveComponent.SetSimulatePhysics` _mainmash false)
  (`SceneComponent.K2_DetachFromComponent` _mainmash "KeepWorld" "KeepWorld" "KeepWorld" true)
  (set `self.BeforeAction` (`SceneComponent.K2_GetComponentToWorld` _mainmash))
  (if (`self.Accurate`)
    (bind (_direction _newtrack_0) (`Timeline|Timeline_In` :!via `PlayFromStart` :!label _label_8)
      (:`Update`
        (`SceneComponent.K2_SetWorldLocationAndRotation` _mainmash (`KismetMathLibrary.VLerp` _beforeaction_location (`self.AttachLocation`) _newtrack_0) (`KismetMathLibrary.RLerp` _beforeaction_rotation (`SceneComponent.K2_GetComponentRotation` (`PlayerCameraManager.TransformComponent` (`GameplayStatics.GetPlayerCameraManager` 0))) _newtrack_0 true) true false))
      (:`Finished`
        (`self.K2_SetActorLocationAndRotation` (.location (`SceneComponent.K2_GetComponentToWorld` (`self.MainMash`))) (.rotation (`SceneComponent.K2_GetComponentToWorld` (`self.MainMash`))) false true :!label _label_9) ; move the actor to the mash
        (`SceneComponent.K2_AttachToComponent` _mainmash_2 (`self.DefaultSceneRoot`) "None" "KeepWorld" "KeepWorld" "KeepWorld" true)
        ;;;[1 1 1] PP Effect On
        (`PrimitiveComponent.SetRenderCustomDepth` _mainmash_2 true)
        (set `PostProcessVolume.bEnabled` true (`/Game/PhysicalS/BP/Character/PC_PIS.PP_Playroom` (cast `/Game/PhysicalS/BP/Character/PC_PIS` (`GameplayStatics.GetPlayerController` 0) :!pure true)))
        (set `self.Rotate` true)))
    (else
      (cast `/Game/PhysicalS/BP/BP_PickUp_Hard` self
        (:`then`
          (goto _label_9))
        (:`CastFailed`
          (goto _label_8 :!via `PlayFromStart`))))))

(event `Turn`
  (params (DeltaX :type "Float (double-precision)"))
  ;[1 1 1] Rotate/Inspection
  ;;[1 1 1] InputMouse
  (if (`self.Rotate`)
    (`SceneComponent.K2_AddWorldRotation` (`self.MainMash`) (`KismetMathLibrary.MakeRotator` 0.0 0.0 (* DeltaX -1.0)) false false)))

(event `InputAxis|Turn` :consume false
  (params (AxisValue :type "Float (single-precision)"))
  ;[1 1 1] Rotate/Inspection
  ;;[1 1 1] InputMouse
  (`self.Turn` AxisValue))

(event `InputTouch` :consume false
  (params (Location :type "Vector Structure") (FingerIndex :type "ETouchIndex Enum"))
  (bind _y (.y Location))
  ;[1 1 1] Rotate/Inspection
  ;;[1 1 1] Touchscreen
  (:`Moved`
    (`/Engine/EditorBlueprintResources/StandardMacros.FlipFlop`
      (:`A`
        (bind _output_get (set `self.PrevY` _y)))
      (:`B`
        _))
    (`self.LookUp` (* (- _y _output_get) 0.5))))

(event `InputTouch` :consume false
  (params (Location :type "Vector Structure") (FingerIndex :type "ETouchIndex Enum"))
  (bind _x (.x Location))
  ;[1 1 1] Rotate/Inspection
  ;;[1 1 1] Touchscreen
  (:`Moved`
    (`/Engine/EditorBlueprintResources/StandardMacros.FlipFlop`
      (:`A`
        (bind _output_get (set `self.PrevX` _x)))
      (:`B`
        _))
    (`self.Turn` (* (- _x _output_get) 0.5))))

(fn `AttachLocation`
  (returns (ReturnValue :type "Vector Structure"))
  (bind (_offset_x _offset_y _offset_z) (`KismetMathLibrary.BreakVector` (`self.Offset`)))
  (bind _transformcomponent (`PlayerCameraManager.TransformComponent` (`GameplayStatics.GetPlayerCameraManager` 0)))
  (bind _returnvalue (`SceneComponent.K2_GetComponentLocation` _transformcomponent))
  (bind _returnvalue_2 (`SceneComponent.GetForwardVector` _transformcomponent))
  (return (+ _returnvalue (* _returnvalue_2 (`KismetMathLibrary.SelectFloat` (`KismetMathLibrary.Vector_Distance` (- (`SceneComponent.K2_GetComponentLocation` (`self.MainMash`)) (.location (`self.IntTransform`))) _returnvalue) 250.0 (and (`self.IgnoreCamera?`) (not (`TimelineComponent.IsPlaying` (`self.Timeline_In`)))))) (+ (* _returnvalue_2 _offset_x) (* (`SceneComponent.GetRightVector` _transformcomponent) _offset_y) (* (`SceneComponent.GetUpVector` _transformcomponent) _offset_z)))))

(fn `UserConstructionScript`
  (bind _mainmash (`self.MainMash`))
  (bind _sweepmesh (`self.SweepMesh`))
  (set `self.IntTransform` (`SceneComponent.GetRelativeTransform` (`self.MainMash`)))
  ;[1 1 1] Creating a mesh to be moved via "Sweep"
  (if (`self.FixWallPassThrough`)
    (bind _returnvalue (`AddComponent|NODE_AddStaticMeshComponent-0` :`bManualAttachment` true))
    (bind _output_get (set `self.SweepMesh` _returnvalue))
    (`SceneComponent.SetAbsolute` _output_get true true true)
    (`PrimitiveComponent.SetCollisionResponseToChannel` _sweepmesh "ECC_PhysicsBody" "ECR_Ignore")
    (`PrimitiveComponent.SetCollisionResponseToChannel` _sweepmesh "ECC_Pawn" "ECR_Ignore")
    (`SceneComponent.SetVisibility` _sweepmesh false false)
    (`StaticMeshComponent.SetStaticMesh` _sweepmesh (`StaticMeshComponent.StaticMesh` _mainmash))
    (`PrimitiveComponent.SetCollisionEnabled` _sweepmesh "QueryOnly")
    (`SceneComponent.K2_SetWorldTransform` _sweepmesh (`SceneComponent.K2_GetComponentToWorld` _mainmash) false true)
    (for (_array_element _array_index) (`MeshComponent.GetMaterials` _mainmash)
      (`PrimitiveComponent.SetMaterial` _sweepmesh _array_index _array_element))))