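; InputPuzzle_BP is the escape room keypad puzzle that unlocks the door and ends level 1.
; UseKeypad shows the InputPuzzle widget with a back-reference and UI-only input, while CorrectPassword opens DoorBP and sets IsDoorOpen.
; Once open, Tick compares the player controller's location, not the character's, to the door on X or Y.
; A match shows FinishedLevel1 after a delay and pauses, though an author note flags this proximity check as buggy.
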(event `Use Keypad`
  (bind _returnvalue (`GameplayStatics.GetPlayerController` 0))
  (bind _returnvalue_2 (`|CreateWidget` "/Game/EscapeRoom/Widgets/InputPuzzle.InputPuzzle_C"))
  (set `/Game/EscapeRoom/Widgets/InputPuzzle.InputPanelBP` self _returnvalue_2)
  (`UserWidget.AddToViewport` _returnvalue_2 0)
  (`WidgetBlueprintLibrary.SetInputMode_UIOnlyEx` _returnvalue _returnvalue_2)
  (set `PlayerController.bShowMouseCursor` true _returnvalue))

(event `Correct Password`
  (`/Game/EscapeRoom/Door_BP.OpenDoor` (`self.DoorBP`))
  (set `self.isDoorOpen` true))

(event `self.ReceiveTick`
  (params (DeltaSeconds :type "Float (single-precision)"))
  (bind (_returnvalue_x _returnvalue_y) (`KismetMathLibrary.BreakVector` (- (`self.K2_GetActorLocation` (`GameplayStatics.GetPlayerController` 0)) (`self.K2_GetActorLocation` (`self.DoorBP`)))))
  ;[1 1 1] bug -> want to make it so that the level complete scene only comes up when you go through the door, but the difference in location between you and the door does not been update constantly
  (if (`self.isDoorOpen`)
    (if (or (< (`KismetMathLibrary.Abs` _returnvalue_x) 10.0) (< (`KismetMathLibrary.Abs` _returnvalue_y) 10.0))
      (bind _asthird_person_character (cast `/Game/ThirdPersonBP/Blueprints/ThirdPersonCharacter` (`GameplayStatics.GetPlayerCharacter` 0)))
      (`KismetSystemLibrary.Delay` 5.0)
      ;;[1 1 1] Level Complete Scene
      (bind _returnvalue (`|CreateWidget` "/Game/EscapeRoom/Widgets/FinishedLevel1.FinishedLevel1_C"))
      (`UserWidget.AddToViewport` _returnvalue 0)
      (set `PlayerController.bShowMouseCursor` true (`GameplayStatics.GetPlayerController` 0))
      (`GameplayStatics.SetGamePaused` true)
      (set `/Game/ThirdPersonBP/Blueprints/ThirdPersonCharacter.PuzzleText` "" _asthird_person_character))))

(fn `UserConstructionScript`)